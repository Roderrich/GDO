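; BP_Platform is a recycled track segment for the endless runner that leapfrogs forward along X when the player enters its trigger box.
; After a short delay it lays a row of pickups, taken from the player character's object pool component, and tells its Manager to spawn obstacles at the new location.
; A Triggered flag blocks repeat overlaps until Reset clears it a tick later.
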(event OnComponentBeginOverlap(Box)
  (params (OverlappedComponent :type Primitive%20Component%20Object%20Reference) (OtherActor :type Actor%20Object%20Reference) (OtherComp :type Primitive%20Component%20Object%20Reference) (OtherBodyIndex :type Integer) (bFromSweep :type Boolean) (SweepResult :type Hit%20Result%20Structure%20%28by%20ref%29))
  (Utilities|Casting|CastToBP_ThirdPersonCharacter OtherActor)
  (if (not (Variables|Default|GetTriggered))
    (Variables|Default|SetTriggered true)
    (Transformation|SetActorLocation (+ (Transformation|GetActorLocation) "10000.000000,0.000000,0.000000") false false)
    (Utilities|FlowControl|Delay 0.2)
    (CallFunction|MovePickUps)
    (Class|BPISpawn|SpawnObstacle(Message) (Variables|Default|GetManager) (Transformation|GetWorldLocation (Variables|Default|GetCube)))
    (CallFunction|Reset)))

(event Custom|Reset
  (Utilities|FlowControl|DelayUntilNextTick)
  (Variables|Default|SetTriggered false))

(event EventBeginPlay
  (bind _asbp_third_person_character (Utilities|Casting|CastToBP_ThirdPersonCharacter (Game|GetPlayerCharacter 0)))
  (Variables|Default|SetAs%20BP%20Third%20Person%20Character _asbp_third_person_character)
  (Utilities|Casting|CastToGI_EndlessRunner (Game|GetGameInstance)))

(event Collision|EventActorBeginOverlap
  (params (OtherActor :type Actor%20Object%20Reference)))

(event EventTick
  (params (DeltaSeconds :type Float%20%28single-precision%29)))

(event EventSpawnPickups
  (Utilities|FlowControl|DelayUntilNextTick)
  (CallFunction|MovePickUps)
  (Class|BPISpawn|SpawnObstacle(Message) (Variables|Default|GetManager) (Transformation|GetWorldLocation (Variables|Default|GetCube))))

(fn ConstructionScript)

(fn MovePickUps
  (for _index (range 0 7)
    ;[0.15 0.15 0.15 0.5] Get objects from the object pool and use set them
    (bind _output_get (Default|GetObject (Variables|/Game/ThirdPerson/Blueprints/BP_ThirdPersonCharacter.BP_ThirdPersonCharacter_C|GetBPC_Pool_Pickup (Variables|Default|GetAs%20BP%20Third%20Person%20Character))))
    (Transformation|SetActorLocation _output_get (+ (- (Transformation|GetWorldLocation (Variables|Default|GetCube)) "1000.000000,0.000000,0.000000") (Math|Vector|MakeVector (* (+ _index 1) 300) 0.0 1.5e+02)) false true))
  (return))