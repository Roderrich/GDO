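; Obstacle manager for the endless runner that places obstacles around a requested location.
; On BeginPlay it caches the third-person game mode, whose random stream drives the placement.
; SpawnObstacle calls GetP, which repeatedly takes a pickup from the BPCObstacle component and teleports it to a stepped random X offset, raised slightly above that location.
; UseSeed is an empty stub.
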(event EventBeginPlay
  (bind _asbp_third_person_game_mode (Utilities|Casting|CastToBP_ThirdPersonGameMode (Game|GetGameMode)))
  (Variables|Default|SetAs%20BP%20Third%20Person%20Game%20Mode _asbp_third_person_game_mode))

(event Collision|EventActorBeginOverlap
  (params (OtherActor :type Actor%20Object%20Reference)))

(event EventTick
  (params (DeltaSeconds :type Float%20%28single-precision%29)))

(event EventSpawnObstacle
  (params (Location :type Vector :default "0, 0, 0"))
  (CallFunction|GetP Location))

(fn ConstructionScript)

(fn GetP
  (params (Location :type Vector))
  (for _index (range 0 3)
    (bind _output_get (Default|GetPickup (Variables|Default|GetBPC_Obstacle)))
    (Transformation|SetActorLocation _output_get (+ Location (Math|Vector|MakeVector (* (Math|Random|RandomIntegerinRangefromStream (Variables|/Game/ThirdPerson/Blueprints/BP_ThirdPersonGameMode.BP_ThirdPersonGameMode_C|GetStream (Variables|Default|GetAs%20BP%20Third%20Person%20Game%20Mode)) -5 5) 500) 0.0 1e+02)) false true)))

(fn UseSeed
  (return ""))