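; BP_Enemy is an enemy actor for the endless runner game.
; On BeginPlay it calls its parent and sets its ID to 1.
; Any damage teleports it to the world origin and clears its InUse flag instead of destroying it, which suggests it is recycled through an object pool.
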(event EventBeginPlay
  (|CallParentFunction)
  (Variables|Default|SetID 1))

(event Collision|EventActorBeginOverlap
  (params (OtherActor :type Actor%20Object%20Reference))
  (|CallParentFunction OtherActor) ; This node is disabled and will not be called.\nDrag off pins to build functionality.
)

(event EventTick
  (params (DeltaSeconds :type Float%20%28single-precision%29))
  (|CallParentFunction DeltaSeconds) ; This node is disabled and will not be called.\nDrag off pins to build functionality.
)

(event Game|Damage|EventAnyDamage
  (params (Damage :type Float%20%28single-precision%29) (DamageType :type Damage%20Type%20Object%20Reference) (InstigatedBy :type Controller%20Object%20Reference) (DamageCauser :type Actor%20Object%20Reference))
  (Transformation|SetActorLocation "0, 0, 0" false true)
  (Variables|Default|SetInUse false))

(fn ConstructionScript
  (|CallParentFunction))