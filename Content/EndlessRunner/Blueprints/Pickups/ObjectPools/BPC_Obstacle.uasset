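; Object pool component for the endless runner that hands out reusable obstacles and enemies.
; GetObject scans ObjectPool through message calls for the first free ID 0 entry, marks it in use and returns it.
; GetEnemy does the same for ID 1, but only searches on a 20% roll from the game instance's random stream.
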(event EventBeginPlay
  (|CallParentFunction) ; This node is disabled and will not be called.\nDrag off pins to build functionality.
)

(event EventTick
  (params (DeltaSeconds :type Float%20%28single-precision%29))
  (|CallParentFunction DeltaSeconds) ; This node is disabled and will not be called.\nDrag off pins to build functionality.
)

(fn GetObject
  (for (_array_element _array_index) (Variables|Default|GetObjectPool)
    ;[0.15 0.15 0.15 0.5] Compares the Chosen Object's ID with the Required ID
    (bind _id (Class|BPICheckObject|CheckID(Message) _array_element))
    (if (== _id 0)
      ;[0.15 0.15 0.15 0.5] Check if the Object Is already In Use
      (bind _newparam (Class|BPICheckObject|CheckUse(Message) _array_element))
      (if (not _newparam)
        (Class|BPICheckObject|SetUse(Message) (Utilities|Array|Get(acopy) (Variables|Default|GetObjectPool) _array_index))
        (bind _output_get (LocalVariables|SetObstacleObject (Utilities|Array|Get(acopy) (Variables|Default|GetObjectPool) _array_index)))
        (return _output_get)))))

(fn GetEnemy
  (if (> (Math|Random|RandomIntegerinRangefromStream (Variables|/Game/EndlessRunner/GI_EndlessRunner.GI_EndlessRunner_C|GetStream (Variables|Default|GetAs%20GI%20Endless%20Runner)) 0 99) 79)
    (for (_array_element _array_index) (Variables|Default|GetObjectPool)
      ;[0.15 0.15 0.15 0.5] Compares the Chosen Object's ID with the Required ID
      (bind _id (Class|BPICheckObject|CheckID(Message) _array_element))
      (if (== _id 1)
        ;[0.15 0.15 0.15 0.5] Check if the Object Is already In Use
        (bind _newparam (Class|BPICheckObject|CheckUse(Message) _array_element))
        (if (not _newparam)
          (Class|BPICheckObject|SetUse(Message) (Utilities|Array|Get(acopy) (Variables|Default|GetObjectPool) _array_index))
          (bind _output_get (LocalVariables|SetNewLocalVar (Utilities|Array|Get(acopy) (Variables|Default|GetObjectPool) _array_index)))
          (return _output_get))))))