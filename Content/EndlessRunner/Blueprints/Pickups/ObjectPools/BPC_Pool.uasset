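; Actor component that acts as an object pool for pickups in the endless runner.
; BeginPlay caches the game instance and calls Pool, which gathers placed actors of the Actor class, though Actor is set to BP_Pickup only afterward.
; GetObject returns the first pooled object not flagged in use and marks it used through message calls, without removing it.
; ReturnObject is an empty stub.
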(event Custom|Pool
  ;[0.15 0.15 0.15 0.5] Get all valid actors and collect them into one array
  (bind _actor (Variables|Default|GetActor)
    (:then
      (bind _outactors (Actor|GetAllActorsOfClass _actor))
      (for _array_element _outactors
        (Utilities|Array|Add (Variables|Default|GetObjectPool) _array_element)))
    (:else)))

(event EventBeginPlay
  (bind _asgi_endless_runner (Utilities|Casting|CastToGI_EndlessRunner (Game|GetGameInstance)))
  (Variables|Default|SetAs%20GI%20Endless%20Runner _asgi_endless_runner)
  (CallFunction|Pool)
  (Variables|Default|SetActor "/Game/EndlessRunner/Blueprints/Pickups/BP_Pickup.BP_Pickup_C"))

(event EventTick
  (params (DeltaSeconds :type Float%20%28single-precision%29)))

(fn GetObject
  ;[0.15 0.15 0.15 0.5] Gets last element of array and removes it for use
  (for (_array_element _array_index) (Variables|Default|GetObjectPool)
    (bind _newparam (Class|BPICheckObject|CheckUse(Message) _array_element))
    (Class|BPICheckObject|CheckID(Message) _array_element)
    (if (not _newparam)
      (Class|BPICheckObject|SetUse(Message) (Utilities|Array|Get(acopy) (Variables|Default|GetObjectPool) _array_index))
      (bind _output_get (LocalVariables|SetNewLocalVar (Utilities|Array|Get(acopy) (Variables|Default|GetObjectPool) _array_index)))
      (return _output_get))))

(fn ReturnObject)