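; Object pool component for endless runner pickups that hands out a free pickup of a randomly chosen type.
; ChoosePickup makes a weighted roll for one of three IDs, heavily favouring the first, using the game instance's random stream.
; GetObject scans the inherited pool through message calls for the first unused match, flags it in use and returns it.
; An older inline selection branch in GetObject is left disconnected.
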(event EventBeginPlay
  (|CallParentFunction))

(event EventTick
  (params (DeltaSeconds :type Float%20%28single-precision%29))
  (|CallParentFunction DeltaSeconds))

(fn GetObject
  (bind _newparam (CallFunction|ChoosePickup))
  (for (_array_element _array_index) (Variables|Default|GetObjectPool)
    ;[0.15 0.15 0.15 0.5] Compares the Chosen Object's ID with the Required ID
    (bind _id (Class|BPICheckObject|CheckID(Message) _array_element))
    (if (== _id _newparam)
      ;[0.15 0.15 0.15 0.5] Check if the Object Is already In Use
      (bind _newparam_2 (Class|BPICheckObject|CheckUse(Message) _array_element))
      (if (not _newparam_2)
        (Class|BPICheckObject|SetUse(Message) (Utilities|Array|Get(acopy) (Variables|Default|GetObjectPool) _array_index))
        (bind _output_get (LocalVariables|SetNewLocalVar (Utilities|Array|Get(acopy) (Variables|Default|GetObjectPool) _array_index)))
        (return _output_get)))))

(fn ChoosePickup
  ;[0.15 0.15 0.15 0.5] Chooses a pickup through their designated probability
  (if (> (Math|Random|RandomIntegerinRangefromStream (Variables|/Game/EndlessRunner/GI_EndlessRunner.GI_EndlessRunner_C|GetStream (Variables|Default|GetAs%20GI%20Endless%20Runner)) 0 99) 87)
    (if (> (Math|Random|RandomIntegerinRangefromStream (Variables|/Game/EndlessRunner/GI_EndlessRunner.GI_EndlessRunner_C|GetStream (Variables|Default|GetAs%20GI%20Endless%20Runner)) 0 12) 11)
      (return 2)
      (else
        (return 1)))
    (else
      (return 0))))