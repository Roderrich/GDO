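; Component that pools pickup actors for the endless runner so they can be reused.
; On BeginPlay it gathers every existing actor of a configurable class into an ObjectPool array, without spawning any.
; GetPickup returns the first entry whose CheckMessage is false and flags it through SetUseMessage, leaving it in the array despite its comment.
; ReturnPickup is an empty stub.
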(event Custom|Pool
  ;[0.15 0.15 0.15 0.5] Get all valid actors and collect them into one array
  (bind _actor (Variables|Default|GetActor)
    (:then
      (bind _outactors (Actor|GetAllActorsOfClass _actor))
      (for _array_element _outactors
        (Utilities|Array|Add (Variables|Default|GetObjectPool) _array_element)))
    (:else)))

(event EventBeginPlay
  (CallFunction|Pool))

(event EventTick
  (params (DeltaSeconds :type Float%20%28single-precision%29)))

(fn GetPickup
  ;[0.15 0.15 0.15 0.5] Gets last element of array and removes it for use
  (for (_array_element _array_index) (Variables|Default|GetObjectPool)
    (bind _newparam (Class|BPICheck|Check(Message) _array_element))
    (if (not _newparam)
      (Class|BPICheck|SetUse(Message) (Utilities|Array|Get(acopy) (Variables|Default|GetObjectPool) _array_index))
      (bind _output_get (LocalVariables|SetNewLocalVar (Utilities|Array|Get(acopy) (Variables|Default|GetObjectPool) _array_index)))
      (return _output_get))))

(fn ReturnPickup)