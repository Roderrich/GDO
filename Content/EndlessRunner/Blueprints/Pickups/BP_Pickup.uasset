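; BP_Pickup is a reusable endless runner pickup identified by an ID.
; When its box overlaps BP_ThirdPersonCharacter, it passes the ID to the character, clears its in-use flag and teleports to a stored location rather than being destroyed.
; SetUse, SetNotUse and CheckUse expose that pool-style state.
; SetID only returns zero, as its per-ID mesh, material and transform logic is disconnected.
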(event OnComponentBeginOverlap(Box)
  (params (OverlappedComponent :type Primitive%20Component%20Object%20Reference) (OtherActor :type Actor%20Object%20Reference) (OtherComp :type Primitive%20Component%20Object%20Reference) (OtherBodyIndex :type Integer) (bFromSweep :type Boolean) (SweepResult :type Hit%20Result%20Structure%20%28by%20ref%29))
  (bind _asbp_third_person_character (Utilities|Casting|CastToBP_ThirdPersonCharacter OtherActor))
  (CallFunction|Pickup _asbp_third_person_character)
  (Variables|Default|SetInuse_0 false)
  (Transformation|SetActorLocation (Variables|Default|GetLocation) false true))

(event EventBeginPlay
  (Variables|Default|SetInuse_0 false))

(event Collision|EventActorBeginOverlap
  (params (OtherActor :type Actor%20Object%20Reference)))

(event EventTick
  (params (DeltaSeconds :type Float%20%28single-precision%29)))

(event EventSetNotUse
  (Variables|Default|SetInuse_0 false)
  (Transformation|SetActorLocation (Variables|Default|GetLocation) false true))

(event EventSetUse
  (Variables|Default|SetInuse_0 true))

(fn ConstructionScript)

(fn Pickup
  (params (Actor :type Actor%20Object%20Reference))
  (Class|BPIPickups|Pickuped(Message) Actor (Variables|Default|GetID)))

(fn Return)

(fn CheckID
  (return (Variables|Default|GetID)))

(fn CheckUse
  (return (Variables|Default|GetInuse_0)))

(fn SetID
  (params (NewParam :type Integer))
  (return 0))