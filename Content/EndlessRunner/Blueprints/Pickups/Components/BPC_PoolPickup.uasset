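; BPC_PoolPickup is an object pool component for pickups in an endless runner.
; On BeginPlay it gathers every actor of the configured Pickup class already in the level into ObjectPool, rather than spawning them.
; GetPickup pops the last pooled actor, records it in UsedObjectPool and returns it, provided the pool is not empty.
; The file contains no logic for returning used pickups to the pool.
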(event Custom|Pool
  ;[0.15 0.15 0.15 0.5] Get all valid actors and collect them into one array
  (bind _pickup (Variables|Default|GetPickup)
    (:then
      (bind _outactors (Actor|GetAllActorsOfClass _pickup))
      (for _array_element _outactors
        (Utilities|Array|Add (Variables|Default|GetObjectPool) _array_element)))
    (:else)))

(event EventBeginPlay
  (CallFunction|Pool))

(event EventTick
  (params (DeltaSeconds :type Float%20%28single-precision%29)))

(fn GetPickup
  (bind _objectpool (Variables|Default|GetObjectPool))
  (bind _returnvalue (Utilities|Array|LastIndex _objectpool))
  ;[0.15 0.15 0.15 0.5] Gets last element of array and removes it for use
  (if (> (Utilities|Array|Length _objectpool) 0)
    (LocalVariables|SetNewLocalVar (Utilities|Array|Get(acopy) _objectpool _returnvalue))
    (Utilities|Array|RemoveIndex (Variables|Default|GetObjectPool) _returnvalue)
    (Utilities|Array|Add (Variables|Default|GetUsedObjectPool) (LocalVariables|GetNewLocalVar))
    (return (LocalVariables|GetNewLocalVar))))