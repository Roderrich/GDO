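; Obstacle Blueprint for the endless runner's pickups, extending a parent class whose GetPickup it passes through unchanged.
; ChooseObstacle rolls on the game mode's random stream and, 20% of the time, scans ObjectPool through message calls for unused ID 1 entries.
; It marks every match as used, without stopping at the first, and only prints each name, with no spawning or placement.
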(event EventBeginPlay
  (|CallParentFunction) ; This node is disabled and will not be called.\nDrag off pins to build functionality.
)

(event EventTick
  (params (DeltaSeconds :type Float%20%28single-precision%29))
  (|CallParentFunction DeltaSeconds) ; This node is disabled and will not be called.\nDrag off pins to build functionality.
)

(fn GetPickup
  (bind _output_get (|CallParentFunction))
  (return _output_get))

(fn ChooseObstacle
  (if (> (Math|Random|RandomIntegerinRangefromStream (Variables|/Game/ThirdPerson/Blueprints/BP_ThirdPersonGameMode.BP_ThirdPersonGameMode_C|GetStream (Variables|Default|GetAs%20BP%20Third%20Person%20Game%20Mode)) 0 99) 79)
    (for (_array_element _array_index) (Variables|Default|GetObjectPool)
      (bind _id (Class|BPICheckObject|CheckID(Message) _array_element))
      (if (== _id 1)
        (bind _newparam (Class|BPICheckObject|CheckUse(Message) _array_element))
        (if (not _newparam)
          (Class|BPICheckObject|SetUse(Message) (Utilities|Array|Get(acopy) (Variables|Default|GetObjectPool) _array_index))
          (bind _output_get (LocalVariables|SetNewLocalVar (Utilities|Array|Get(acopy) (Variables|Default|GetObjectPool) _array_index)))
          (Development|PrintString (Utilities|GetDisplayName _output_get) true true "(R=0.000000,G=0.000000,B=0.000000,A=1.000000)"))))))